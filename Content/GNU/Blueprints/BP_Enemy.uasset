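; BP_Enemy is a damageable enemy that attacks on a looping timer and shows a health bar widget.
; Each attack sphere-traces forward against WorldStatic objects, sends damage to the hit actor and spawns an explosion on success.
; Health, healing and damage calls forward to BPCDamageSystem, while shield functions return zero.
; Component events are bound in the construction script; death ragdolls the mesh, while block and damage responses only print.
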(event `self.ReceiveBeginPlay`
  (`KismetSystemLibrary.K2_SetTimerDelegate` (delegate `Attack`) 2.0 true)
  (bind _returnvalue (`|CreateWidget` "/Game/GNU/Skills/W_HealtchBar.W_HealtchBar_C" null self))
  (`WidgetComponent.SetWidget` (`self.Widget`) _returnvalue))

(event `self.ReceiveTick`
  (params (DeltaSeconds :type "Float (single-precision)")))

(event `Attack`
  (bind _returnvalue (`self.K2_GetActorLocation`))
  (bind (_outhit _returnvalue_2) (`KismetSystemLibrary.SphereTraceSingleForObjects` :`Start` _returnvalue :`End` (+ _returnvalue (* (`self.GetActorForwardVector`) 100.0)) :`Radius` 20.0 :`ObjectTypes` (`|MakeArray` "ObjectTypeQuery1" :!type "EObjectTypeQuery Enum") :`DrawDebugType` "ForDuration" :`TraceColor` (struct :`R` 1.0 :`B` 0.736737 :`A` 1.0) :`TraceHitColor` (struct :`R` 0.534968 :`G` 0.879147 :`B` 1.0 :`A` 1.0) :`DrawTime` 1.0))
  (if _returnvalue_2
    (bind (_bblockinghit _binitialoverlap _time _distance _location _impactpoint _normal _impactnormal _physmat _hitactor) (`GameplayStatics.BreakHitResult` _outhit))
    (bind _wasdamaged (message `/Game/GNU/Skills/DamageSystem/BPI_Damagable.TakeDamage` _hitactor (make `/Game/GNU/Skills/DamageSystem/S_DamageInfo` 10.0 "NewEnumerator1" "NewEnumerator1")))
    (if _wasdamaged
      (`GameplayStatics.SpawnEmitterAtLocation` "/Game/FXVarietyPack/Particles/P_ky_explosion.P_ky_explosion" _location))))

(event `Death`
  (bind _mesh (`self.Mesh`))
  (`PrimitiveComponent.SetSimulatePhysics` _mesh true)
  (`PrimitiveComponent.SetCollisionEnabled` _mesh "QueryAndPhysics"))

(event `Blocked`
  (params (CanBeParried :type Boolean))
  (`KismetSystemLibrary.PrintString` "Blocked"))

(event `DamgaeResponse`
  (params (DamageResponse :type "/Game/GNU/Skills/DamageSystem/E_DamageResponse Enum" :default "NewEnumerator0"))
  (`KismetSystemLibrary.PrintString` (`|GetEnumeratorNameAsString` DamageResponse)))

(fn `GetCurrentHealth`
  (returns (Health :type "Float (double-precision)"))
  (return (`/Game/GNU/Skills/DamageSystem/BPC_DamageSystem.Health` (`self.BPC_DamageSystem`))))

(fn `GetCurrentShield`
  (returns (Shield :type "Float (double-precision)"))
  (return 0.0))

(fn `GetMaxHealth`
  (returns (MaxHealth :type "Float (double-precision)"))
  (return (`/Game/GNU/Skills/DamageSystem/BPC_DamageSystem.MaxHealth` (`self.BPC_DamageSystem`))))

(fn `GetMaxShield`
  (returns (MaxShield :type "Float (double-precision)"))
  (return 0.0))

(fn `Heal`
  (params (Amount :type "Float (double-precision)"))
  (returns (NewHealth :type "Float (double-precision)"))
  (bind _newhealth (`/Game/GNU/Skills/DamageSystem/BPC_DamageSystem.Heal` (`self.BPC_DamageSystem`) Amount))
  (return _newhealth))

(fn `Shield`
  (params (Amount :type "Float (double-precision)"))
  (returns (NewShield :type "Float (double-precision)"))
  (return 0.0))

(fn `TakeDamage`
  (params (DamageInfo :type "/Game/GNU/Skills/DamageSystem/S_DamageInfo Structure"))
  (returns (WasDamaged :type Boolean))
  (bind _wasdamaged (`/Game/GNU/Skills/DamageSystem/BPC_DamageSystem.TakeDamage` (`self.BPC_DamageSystem`) DamageInfo))
  (return _wasdamaged))

(fn `UserConstructionScript`
  (bind _bpc_damagesystem (`self.BPC_DamageSystem`))
  (add `/Game/GNU/Skills/DamageSystem/BPC_DamageSystem.OnDeath` _bpc_damagesystem (`|CreateDelegate` :!event `Death`))
  (add `/Game/GNU/Skills/DamageSystem/BPC_DamageSystem.OnBlock` _bpc_damagesystem (`|CreateDelegate` :!event `Blocked`))
  (add `/Game/GNU/Skills/DamageSystem/BPC_DamageSystem.OnDamageResponse` _bpc_damagesystem (`|CreateDelegate` :!event `DamgaeResponse`)))