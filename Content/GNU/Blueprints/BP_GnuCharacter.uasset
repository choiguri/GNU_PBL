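; BP_GnuCharacter is a character Blueprint with a hitscan attack and simple health handling.
; Left click runs a sphere trace along the camera's forward vector against Pawn objects, with debug drawing on, and applies damage to the hit actor.
; Incoming damage reduces Health; at zero or below, movement is disabled and the mesh switches to physics simulation as a ragdoll death.
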(event `self.ReceiveBeginPlay`)

(event `Key|LeftMouseButton`
  (params (Key :type "Key Structure"))
  (bind _camera (`self.Camera`))
  (bind _returnvalue (`SceneComponent.K2_GetComponentLocation` _camera))
  ;[1 1 1] Attack
  (:`Pressed`
    (bind (_outhit _returnvalue_2) (`KismetSystemLibrary.SphereTraceSingleForObjects` :`Start` _returnvalue :`End` (+ _returnvalue (* (`KismetMathLibrary.GetForwardVector` (`SceneComponent.K2_GetComponentRotation` _camera)) 3000.0)) :`Radius` 25.0 :`ObjectTypes` (`|MakeArray` "ObjectTypeQuery3" :!type "EObjectTypeQuery Enum") :`DrawDebugType` "ForDuration" :`DrawTime` 2.0))
    (if _returnvalue_2
      (`GameplayStatics.ApplyDamage` (`.HitActor` (`GameplayStatics.BreakHitResult` _outhit)) 10.0))))

(event `self.ReceiveAnyDamage`
  (params (Damage :type "Float (single-precision)") (DamageType :type "DamageType Object Reference") (InstigatedBy :type "Controller Object Reference") (DamageCauser :type "Actor Object Reference"))
  ;[1 1 1] Health
  (set `self.Health` (- (`self.Health`) Damage))
  (if (<= (`self.Health`) 0.0)
    (`CharacterMovementComponent.DisableMovement` (`self.CharacterMovement`))
    (`PrimitiveComponent.SetSimulatePhysics` (`self.Mesh`) true)))

(fn `UserConstructionScript`)