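; Boss monster character with a mouth attack, a damageable health pool and an on-screen boss health bar, created at BeginPlay and updated every Tick.
; Its Attack event plays a montage guarded by IsAttacking, whose notify fires a debug-drawn forward sphere trace from AttackPos that damages the first Pawn hit.
; Incoming damage lowers Health, and at zero or below the monster stops moving and its mesh switches to physics simulation.
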(event `self.ReceiveBeginPlay`
  ;[1 1 1] HealthBar
  (bind _returnvalue (`|CreateWidget` "/Game/GNU/Monster/BossFight/WB_BossFightHealth.WB_BossFightHealth_C"))
  (`UserWidget.AddToViewport` _returnvalue 0)
  (set `self.HealthUI` _returnvalue))

(event `self.ReceiveTick`
  (params (DeltaSeconds :type "Float (single-precision)"))
  ;[1 1 1] HealthBar
  (`ProgressBar.SetPercent` (`/Game/GNU/Monster/BossFight/WB_BossFightHealth.HealthBar` (`self.HealthUI`)) (/ (`self.Health`) 100.0)))

(event `/Game/GNU/Monster/AI/BPI_BossFight.Attack`
  (bind _attackpos (`self.AttackPos`))
  (bind _returnvalue (`SceneComponent.K2_GetComponentLocation` _attackpos))
  ;[1 1 1] Attack
  (if (not (`self.IsAttacking?`))
    (`|PlayMontage` (`self.Mesh`) "/Game/GNU/Monster/Animation/AttackMouthAnim_Montage.AttackMouthAnim_Montage"
      (:`then`
        (set `self.IsAttacking?` true))
      (:`OnCompleted`
        (set `self.IsAttacking?` false))
      (:`OnNotifyBegin`
        (bind (_outhit _returnvalue_2) (`KismetSystemLibrary.SphereTraceSingleForObjects` :`Start` _returnvalue :`End` (+ _returnvalue (* (`KismetMathLibrary.GetForwardVector` (`SceneComponent.K2_GetComponentRotation` _attackpos)) 3000.0)) :`Radius` 50.0 :`ObjectTypes` (`|MakeArray` "ObjectTypeQuery3" :!type "EObjectTypeQuery Enum") :`DrawDebugType` "ForDuration" :`DrawTime` 2.0))
        (if _returnvalue_2
          (`GameplayStatics.ApplyDamage` (`.HitActor` (`GameplayStatics.BreakHitResult` _outhit)) 10.0))))))

(event `self.ReceiveAnyDamage`
  (params (Damage :type "Float (single-precision)") (DamageType :type "DamageType Object Reference") (InstigatedBy :type "Controller Object Reference") (DamageCauser :type "Actor Object Reference"))
  ;[1 1 1] Health
  (set `self.Health` (- (`self.Health`) Damage))
  (if (<= (`self.Health`) 0.0)
    (`CharacterMovementComponent.DisableMovement` (`self.CharacterMovement`))
    (`PrimitiveComponent.SetSimulatePhysics` (`self.Mesh`) true)))

(fn `UserConstructionScript`)