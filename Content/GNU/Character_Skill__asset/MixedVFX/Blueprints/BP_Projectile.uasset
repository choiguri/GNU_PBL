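; BP_Projectile is a visual effects projectile that takes its look from the player pawn, a BP_MainCamera.
; On BeginPlay it sets its Niagara component to the camera's template at the current NiagaraID.
; When its Box component hits something, it spawns the hit system at the same index, slightly offset along X from the impact, then destroys itself.
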(event `self.ReceiveBeginPlay`
  (bind _asbp_main_camera (cast `/Game/GNU/Character_Skill__asset/MixedVFX/Blueprints/BP_MainCamera` (`GameplayStatics.GetPlayerPawn` 0)))
  (`NiagaraComponent.SetAsset` (`self.Niagara`) (`|GetArrayItem` (`/Game/GNU/Character_Skill__asset/MixedVFX/Blueprints/BP_MainCamera.NiagaraTemplate` _asbp_main_camera) (`KismetMathLibrary.Clamp` (`/Game/GNU/Character_Skill__asset/MixedVFX/Blueprints/BP_MainCamera.NiagaraID` _asbp_main_camera) 0 20)) true))

(event `self.Box.OnComponentHit`
  (params (HitComponent :type "PrimitiveComponent Object Reference") (OtherActor :type "Actor Object Reference") (OtherComp :type "PrimitiveComponent Object Reference") (NormalImpulse :type "Vector Structure") (Hit :type "HitResult Structure (by ref)"))
  (`NiagaraFunctionLibrary.SpawnSystemAtLocation` (`|GetArrayItem` (`/Game/GNU/Character_Skill__asset/MixedVFX/Blueprints/BP_MainCamera.Hits` (stale `self.ReceiveBeginPlay` _asbp_main_camera)) (`KismetMathLibrary.Clamp` (`/Game/GNU/Character_Skill__asset/MixedVFX/Blueprints/BP_MainCamera.NiagaraID` (stale `self.ReceiveBeginPlay` _asbp_main_camera)) 0 20)) (`KismetMathLibrary.MakeVector` (- (.x (`.Location` (`GameplayStatics.BreakHitResult` Hit))) 18.0) (.y (`.Location` (`GameplayStatics.BreakHitResult` Hit))) (.z (`.Location` (`GameplayStatics.BreakHitResult` Hit)))))
  (`self.K2_DestroyActor`))

(fn `UserConstructionScript`)