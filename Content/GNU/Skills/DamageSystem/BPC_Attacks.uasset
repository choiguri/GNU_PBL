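; BPC_Attacks is an attack component in the damage system that currently implements one skill, an area heal on a target.
; HealTarget line traces from the target toward its location with Z scaled by -1000 to find the ground, then spawns and triggers BP_Heal at the hit.
; The spawned actor's AOE overlap event calls back into the component, which sends a fixed heal message only if the overlapped actor is the target.
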(event `Heal Target`
  (params (`Heal Target` :type "Actor Object Reference"))
  (bind _returnvalue (`Actor.K2_GetActorLocation` `Heal Target`))
  (`/Engine/EditorBlueprintResources/StandardMacros.IsValid` `Heal Target`
    (:`Is Valid`
      (bind (_outhit _returnvalue_2) (`KismetSystemLibrary.LineTraceSingle` _returnvalue (* _returnvalue (1.0 1.0 -1000.0)) "TraceTypeQuery1" false (`|MakeArray` `Heal Target`)))
      (if _returnvalue_2
        (bind _returnvalue_3 (`|SpawnActorFromClass` "/Game/GNU/Skills/BP_Heal.BP_Heal_C" (`KismetMathLibrary.MakeTransform` (`.Location` (`GameplayStatics.BreakHitResult` _outhit))) "Undefined" "MultiplyWithRoot" null false true false null))
        (add `/Game/GNU/Skills/BP_Skill_Base.OnAOEOverlapActor` _returnvalue_3 (delegate `OnHealTarget`))
        (`/Game/GNU/Skills/BP_Skill_Base.Trigger` _returnvalue_3)))))

(event `OnHealTarget`
  (params (Actor :type "Actor Object Reference"))
  (if (== Actor (stale `Heal Target` `Heal Target`))
    (message `/Game/GNU/Skills/DamageSystem/BPI_Damagable.Heal` Actor 10.0)))