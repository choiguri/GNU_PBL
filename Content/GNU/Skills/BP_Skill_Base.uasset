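; BP_Skill_Base is a base skill actor that provides an area-of-effect hit check around its location.
; Trigger, optionally fired one second after BeginPlay, runs a sphere overlap for pawns, optionally ignoring the instigator.
; Each actor found is broadcast through the OnAOEOverlapActor dispatcher and its name is printed.
; A debug sphere draw exists in the graph but is not connected.
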(event `self.ReceiveBeginPlay`
  (if (`self.TriggerOnBeginPlay`)
    (`KismetSystemLibrary.Delay` 1.0)
    (`self.Trigger`)))

(event `Trigger`
  (`self.SpawnAOESphere`))

(event `SpawnAOESphere`
  (bind _outactors (`KismetSystemLibrary.SphereOverlapActors` (`self.K2_GetActorLocation`) (`self.Sphere Radius`) (`|MakeArray` "ObjectTypeQuery3" :!type "EObjectTypeQuery Enum") null (select `bool` (`self.IgnoreInstigator`) :`true` (`|MakeArray` (`self.GetInstigator`) :!type "Actor Object Reference"))))
  (for _array_element _outactors
    (`self.OnAOEOverlapActor` _array_element)
    (`KismetSystemLibrary.PrintString` (`KismetSystemLibrary.GetDisplayName` _array_element))))

(fn `UserConstructionScript`)