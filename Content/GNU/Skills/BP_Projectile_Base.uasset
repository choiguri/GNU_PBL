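; Base projectile Blueprint for skills that flies at a set speed and gravity, optionally homing on a Target.
; The construction script configures ProjectileMovement, and BeginPlay aims velocity at a valid Target and makes the box collision ignore the instigator, or the owner if none.
; A hit only destroys the actor; impact callback, effect and sound calls exist but are not wired to run.
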(event `self.ReceiveBeginPlay`
  (bind _returnvalue (`self.GetInstigator`))
  (`self.Rotator To Target`)
  (`PrimitiveComponent.IgnoreActorWhenMoving` (`self.BoxCollision`) (select `bool` (`KismetSystemLibrary.IsValid` _returnvalue) :`false` (`self.GetOwner`) :`true` _returnvalue :!type "Actor Object Reference") true))

(event `Rotator To Target`
  (`self.Target`
    (:`then`
      (set `MovementComponent.Velocity` (* (`KismetMathLibrary.GetDirectionUnitVector` (`self.K2_GetActorLocation`) (`self.K2_GetActorLocation` (`self.Target`))) (`self.speed`)) (`self.ProjectileMovement`)))
    (:`else`)))

(event `self.BoxCollision.OnComponentHit`
  (params (HitComponent :type "PrimitiveComponent Object Reference") (OtherActor :type "Actor Object Reference") (OtherComp :type "PrimitiveComponent Object Reference") (NormalImpulse :type "Vector Structure") (Hit :type "HitResult Structure (by ref)"))
  (`self.K2_DestroyActor`))

(event `SpawnImpactEffect`
  (params (Location :type "Vector Structure"))
  (bind _impact_effect (`self.Impact Effect`)
    (:`then`
      (`NiagaraFunctionLibrary.SpawnSystemAtLocation` _impact_effect Location))
    (:`else`)))

(fn `UserConstructionScript`
  (bind _projectilemovement (`self.ProjectileMovement`))
  (set `ProjectileMovementComponent.InitialSpeed` (`self.speed`) _projectilemovement)
  (set `ProjectileMovementComponent.MaxSpeed` (`self.speed`) _projectilemovement)
  (set `ProjectileMovementComponent.ProjectileGravityScale` (`self.gravity`) _projectilemovement)
  (`self.Target`
    (:`then`
      (if (`self.IsHoming`)
        (set `ProjectileMovementComponent.bIsHomingProjectile` true _projectilemovement)
        (set `ProjectileMovementComponent.HomingTargetComponent` (`Actor.RootComponent` (`self.Target`)) _projectilemovement)))
    (:`else`)))