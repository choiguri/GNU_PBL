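; BP_Shoot is an actor in the GrenadeEMP VFX folder that automatically fires projectiles on a repeating loop.
; Each shot spawns a scaled-down ProjectileBP along the Arrow component's rotation, plus a particle system offset from the actor.
; After a random delay, NextArrow plays the NSBeforeShoot effect, waits briefly and fires again, calling itself to continue.
; BeginPlay joins the loop after a short delay, so the first shot skips the pre-shoot effect.
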(event `NextArrow`
  (bind _returnvalue (`self.K2_GetActorLocation`))
  (bind (_returnvalue_location _returnvalue_rotation) (`KismetMathLibrary.BreakTransform` (`SceneComponent.K2_GetComponentToWorld` (`self.Arrow`))))
  (`NiagaraFunctionLibrary.SpawnSystemAtLocation` (`self.NS_BeforeShoot`) (`self.K2_GetActorLocation`))
  (`KismetSystemLibrary.Delay` 1.0)
  (`|SpawnActorFromClass` (`self.Projectile BP`) (`KismetMathLibrary.MakeTransform` _returnvalue _returnvalue_rotation (0.1 0.1 0.1)) "Undefined" "SelectDefaultAtRuntime" null null :!label _label)
  (`NiagaraFunctionLibrary.SpawnSystemAtLocation` null (+ _returnvalue (50.0 0.0 0.0)) (struct :`Pitch` 90.0 :`Roll` 90.0))
  (`KismetSystemLibrary.Delay` (`KismetMathLibrary.RandomFloatInRange` 5.0 4.0))
  (`self.NextArrow`))

(event `self.ReceiveBeginPlay`
  (`KismetSystemLibrary.Delay` 1.0)
  (goto _label))

(fn `UserConstructionScript`)