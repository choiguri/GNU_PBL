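; Brown EMP grenade projectile that detonates once hits on its collision sphere bring its Health down to zero or below.
; Detonation stops the trail Niagara and movement, enlarges the sphere and disables its collision.
; A cast effect spawns just above the impact, then after a delay the EMP effect plays and damages only the hit actor.
; Parallel delayed branches then destroy the projectile.
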(event `self.SphereCollision.OnComponentHit`
  (params (HitComponent :type "PrimitiveComponent Object Reference") (OtherActor :type "Actor Object Reference") (OtherComp :type "PrimitiveComponent Object Reference") (NormalImpulse :type "Vector Structure") (Hit :type "HitResult Structure (by ref)"))
  (bind (_returnvalue_roll _returnvalue_pitch _returnvalue_yaw) (`KismetMathLibrary.BreakRotator` (`self.K2_GetActorRotation`)))
  (bind _spherecollision (`self.SphereCollision`))
  (bind _returnvalue (+ (`.Location` (`GameplayStatics.BreakHitResult` Hit)) (0.0 0.0 60.0)))
  (bind _output_get (set `self.health` (- (`self.health`) 1)))
  (`/Engine/EditorBlueprintResources/StandardMacros.CompareInt` 0 _output_get
    (:`>`
      _)
    (:`==`
      _))
  (`|ExecutionSequence`
    (:`then_0`
      (`ActorComponent.Deactivate` (`self.Niagara`))
      (`PrimitiveComponent.SetSimulatePhysics` _spherecollision false)
      (`SphereComponent.SetSphereRadius` _spherecollision 300.0 true)
      (`PrimitiveComponent.SetCollisionEnabled` _spherecollision "NoCollision")
      (`SceneComponent.SetVisibility` _spherecollision true false)
      (`KismetSystemLibrary.Delay` 4.0)
      (`self.K2_DestroyActor`))
    (:`then_1`
      (`ActorComponent.Deactivate` (`self.ProjectileMovement`))
      (`NiagaraFunctionLibrary.SpawnSystemAtLocation` "/Game/GNU/Character/Skills/GrenadeEMP_vfx/Niagara/EMP_Brown/NS_EMP_Cast_Brown.NS_EMP_Cast_Brown" _returnvalue (`KismetMathLibrary.MakeRotator` (`KismetMathLibrary.RandomFloatInRange` _returnvalue_roll) (`KismetMathLibrary.RandomFloatInRange` _returnvalue_pitch) (`KismetMathLibrary.RandomFloatInRange` _returnvalue_yaw)))
      (`KismetSystemLibrary.Delay` 1.2)
      (`NiagaraFunctionLibrary.SpawnSystemAtLocation` "/Game/GNU/Character/Skills/GrenadeEMP_vfx/Niagara/EMP_Brown/NS_EMP_Brown.NS_EMP_Brown" _returnvalue (`self.K2_GetActorRotation`))
      (`GameplayStatics.ApplyDamage` OtherActor 50.0 (`self.GetInstigatorController` (`self.GetOwner`)) null "/Script/Engine.DamageType")
      (`KismetSystemLibrary.Delay` 3.0)
      (`self.K2_DestroyActor`))))

(fn `UserConstructionScript`)